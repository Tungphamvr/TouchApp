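; BP_Controller is a player controller that detects mouse cursor movement.
; Each tick, CheckCursorMovement reads the DPI-scaled mouse position and compares it with the previous one within a small tolerance.
; When the position differs, it calls the CursorHasMoved dispatcher, then stores the current position for the next check.
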(event `self.ReceiveTick`
  (params (DeltaSeconds :type "Float (single-precision)"))
  (`self.CheckCursorMovement`))

(fn `CheckCursorMovement`
  (bind (_locationx _locationy) (`WidgetLayoutLibrary.GetMousePositionScaledByDPI` self))
  (set `self.Mouse_Position_Current` (`KismetMathLibrary.MakeVector2D` _locationx _locationy))
  (if (not (== (`self.Mouse_Position_Current`) (`self.Mouse_Position_Previous`) :`ErrorTolerance` 1.0))
    (`self.Cursor_HasMoved`))
  (set `self.Mouse_Position_Previous` (`self.Mouse_Position_Current`)))

(fn `UserConstructionScript`)